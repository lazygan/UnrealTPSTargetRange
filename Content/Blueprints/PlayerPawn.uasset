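; Player pawn that carries a rifle, fires it and can enter a grenade-holding state.
; On BeginPlay it spawns BP_Rifle onto the mesh's WeaponSocket as the current weapon, caches the hero anim blueprint and shows a crosshair widget.
; Left mouse fires the weapon unless a grenade is held.
; Right mouse sets the grenade flag and ignores move input, while release clears only the flag, without restoring movement.
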(event `Key|RightMouseButton`
  (params (Key :type "Key Structure"))
  (:`Pressed`
    (set `self.holdingGrenade` true)
    (`Controller.SetIgnoreMoveInput` (`GameplayStatics.GetPlayerController` 0) true))
  (:`Released`
    (set `self.holdingGrenade` false)))

(event `Key|LeftMouseButton`
  (params (Key :type "Key Structure"))
  (:`Pressed`
    (if (not (`self.holdingGrenade`))
      (`SWeapon.Fire` (`self.CurrentWeapon`)))))

(event `self.ReceiveBeginPlay`
  (`|ExecutionSequence`
    (:`then_0`
      (bind _returnvalue (`|SpawnActorFromClass` "/Game/Blueprints/BP_Rifle.BP_Rifle_C" (`KismetMathLibrary.MakeTransform` (0.0 0.0 0.0)) "AlwaysSpawn" "OverrideRootScale" self null))
      (set `self.CurrentWeapon` _returnvalue)
      (`self.K2_AttachToComponent` _returnvalue (`self.Mesh`) "WeaponSocket" "SnapToTarget" "SnapToTarget" "SnapToTarget" true))
    (:`then_1`
      (bind _asue4asp_hero_tpp_anim_blueprint (cast `/Game/Blueprints/UE4ASP_HeroTPP_AnimBlueprint` (`SkeletalMeshComponent.GetAnimInstance` (`self.Mesh`))))
      (set `self.As UE4ASP Hero TPP Anim Blueprint` _asue4asp_hero_tpp_anim_blueprint))
    (:`then_2`
      (bind _returnvalue_2 (`|CreateWidget` "/Game/UI/WBP_Crosshair.WBP_Crosshair_C"))
      (`UserWidget.AddToViewport` _returnvalue_2 0))))

(fn `UserConstructionScript`)